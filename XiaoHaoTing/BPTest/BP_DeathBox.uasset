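; BP_DeathBox is a death volume that respawns the player when its DeathTrigger component is overlapped.
; On overlap it disables player 0's input without checking which actor entered, then waits briefly.
; If the "check" save slot exists, it moves the character to the location saved in BP_SaveTheGame and restores input.
; Otherwise it opens a level by name.
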(event OnComponentBeginOverlap(DeathTrigger)
  (params (OverlappedComponent :type Primitive%20Component%20Object%20Reference) (OtherActor :type Actor%20Object%20Reference) (OtherComp :type Primitive%20Component%20Object%20Reference) (OtherBodyIndex :type Integer) (bFromSweep :type Boolean) (SweepResult :type Hit%20Result%20Structure%20%28by%20ref%29))
  (bind _ascharacter (Utilities|Casting|CastToCharacter (Game|GetPlayerCharacter 0)))
  (Input|DisableInput _ascharacter (Game|GetPlayerController 0))
  (Utilities|FlowControl|Delay 2.0)
  (bind _returnvalue (SaveGame|DoesSaveGameExist "check"))
  (if _returnvalue
    (bind _returnvalue_2 (SaveGame|LoadGamefromSlot "check"))
    (bind _asbp_save_the_game (Utilities|Casting|CastToBP_SaveTheGame _returnvalue_2))
    (bind _ascharacter_2 (Utilities|Casting|CastToCharacter (Game|GetPlayerCharacter 0)))
    (Transformation|SetActorLocation _ascharacter_2 (Variables|/Game/XiaoHaoTing/BPTest/BP_SaveTheGame.BP_SaveTheGame_C|GetPlayer_locals _asbp_save_the_game) false false)
    (Input|EnableInput _ascharacter_2 (Game|GetPlayerController 0))
    (else
      (Game|OpenLevel(byName) (Variables|Default|GetNewVar_0)))))

(event EventBeginPlay)

(event Collision|EventActorBeginOverlap
  (params (OtherActor :type Actor%20Object%20Reference)))

(event EventTick
  (params (DeltaSeconds :type Float%20%28single-precision%29)))

(fn ConstructionScript)