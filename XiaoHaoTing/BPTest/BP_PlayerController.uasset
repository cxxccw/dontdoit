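; Player controller that sets up the options save game and provides a brightness adjustment event.
; On BeginPlay it loads the "Options" save slot, or creates and saves a new OptionsSave object if none exists.
; AdjustBrightness maps its Brightness value through a Lerp into a Gamma console command string and executes it.
; The loaded options are only stored here, not applied to brightness.
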(event Custom|Adjust%20Brightness
  (Development|ExecuteConsoleCommand (Utilities|String|Append "Gamma " (Utilities|String|ToString(Float) (Math|Float|Lerp 0.5 1e+01 (Variables|VideoSettingVariables|GetBrightness)))) 0))

(event EventBeginPlay
  (CallFunction|OptionsSaveHandler))

(event EventTick
  (params (DeltaSeconds :type Float%20%28single-precision%29)))

(fn ConstructionScript)

(fn OptionsSaveHandler
  (bind _returnvalue (SaveGame|DoesSaveGameExist "Options"))
  (if _returnvalue
    (bind _returnvalue_2 (SaveGame|LoadGamefromSlot "Options"))
    (bind _asoptions_save (Utilities|Casting|CastToOptionsSave _returnvalue_2))
    (Variables|Default|SetOptionsSave _asoptions_save)
    (else
      (bind _returnvalue_3 (SaveGame|CreateSaveGameObject "/Game/XiaoHaoTing/Options/OptionsSave.OptionsSave_C"))
      (bind _output_get (Variables|Default|SetOptionsSave _returnvalue_3))
      (SaveGame|SaveGametoSlot _output_get "Options"))))